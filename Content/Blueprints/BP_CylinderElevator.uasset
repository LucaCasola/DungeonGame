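; BP_CylinderElevator is a lever-gated elevator that runs a raise-and-lower cycle when the third-person character enters its collision sphere.
; The overlap starts a cycle only if LeverActivated is true and CycleComplete shows no cycle is running.
; Latent MoveComponentTo calls move the Cylinder to fixed relative heights, with a pause between raising and lowering.
; The construction script records the Cylinder's starting world Z, though the movement logic does not read it.
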(event OnComponentBeginOverlap(CollisionSphere)
  (params (OverlappedComponent :type Primitive%20Component%20Object%20Reference) (OtherActor :type Actor%20Object%20Reference) (OtherComp :type Primitive%20Component%20Object%20Reference) (OtherBodyIndex :type Integer) (bFromSweep :type Boolean) (SweepResult :type Hit%20Result%20Structure%20%28by%20ref%29))
  (Utilities|Casting|CastToBP_ThirdPersonCharacter OtherActor)
  (if (Variables|Default|GetleverActivated)
    (if (Variables|Default|GetcycleComplete)
      (Variables|Default|SetcycleComplete false)
      (Components|MoveComponentTo (Variables|Default|GetCylinder) (Math|Vector|MakeVector 0.0 0.0 1e+02) "0, 0, 0" false false 5.0 false) ; Raises elevator
      (Utilities|FlowControl|Delay 3.0)
      (Components|MoveComponentTo (Variables|Default|GetCylinder) (Math|Vector|MakeVector 0.0 0.0 -1.6e+02) "0, 0, 0" false false 5.0 false) ; Lowers elevator
      (Variables|Default|SetcycleComplete true))))

(fn ConstructionScript
  (Variables|Default|SetelevatorStartZ (.z (Transformation|GetWorldLocation (Variables|Default|GetCylinder)))))