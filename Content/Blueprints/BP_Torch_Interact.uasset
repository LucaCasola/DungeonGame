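; BP_Torch_Interact is a torch whose point light and fire effect can be switched on and off.
; The LightOn/Off event reads the fire's visibility and sets both components to the opposite state.
; Overlaps on Torch_Collision set PlayerWithinRange while a BP_ThirdPersonCharacter is inside.
; This graph neither reads that flag nor calls the toggle event.
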(event OnComponentBeginOverlap(Torch_Collision)
  (params (OverlappedComponent :type Primitive%20Component%20Object%20Reference) (OtherActor :type Actor%20Object%20Reference) (OtherComp :type Primitive%20Component%20Object%20Reference) (OtherBodyIndex :type Integer) (bFromSweep :type Boolean) (SweepResult :type Hit%20Result%20Structure%20%28by%20ref%29))
  (Utilities|Casting|CastToBP_ThirdPersonCharacter OtherActor)
  (Variables|Default|SetPlayerWithinRange true))

(event OnComponentEndOverlap(Torch_Collision)
  (params (OverlappedComponent :type Primitive%20Component%20Object%20Reference) (OtherActor :type Actor%20Object%20Reference) (OtherComp :type Primitive%20Component%20Object%20Reference) (OtherBodyIndex :type Integer))
  (Utilities|Casting|CastToBP_ThirdPersonCharacter OtherActor)
  (Variables|Default|SetPlayerWithinRange false))

(event Custom|LightOn/Off
  (if (Variables|/Script/Engine.SceneComponent|GetbVisible (Variables|Default|GetP_Torch_Fire))
    (Rendering|SetVisibility (Variables|Default|GetTorch_PointLight) false false)
    (else
      (Rendering|SetVisibility (Variables|Default|GetTorch_PointLight) true false))))

(fn ConstructionScript)