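; BP_Torch_Interact is a torch that the player can switch on and off when standing near it.
; Overlap events on Torch_Collision set PlayerWithinRange when a BP_Knight enters or leaves.
; The SwitchLight event, with no caller in this Blueprint, checks that flag and uses a FlipFlop to alternately show and hide TorchPointLight and PTorchFire, showing them on the first use.
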(event OnComponentBeginOverlap(Torch_Collision)
  (params (OverlappedComponent :type Primitive%20Component%20Object%20Reference) (OtherActor :type Actor%20Object%20Reference) (OtherComp :type Primitive%20Component%20Object%20Reference) (OtherBodyIndex :type Integer) (bFromSweep :type Boolean) (SweepResult :type Hit%20Result%20Structure%20%28by%20ref%29))
  ;[1 1 1] Set "PlayerWithinRange" var
  (Utilities|Casting|CastToBP_Knight OtherActor)
  (Variables|Default|SetPlayerWithinRange true))

(event OnComponentEndOverlap(Torch_Collision)
  (params (OverlappedComponent :type Primitive%20Component%20Object%20Reference) (OtherActor :type Actor%20Object%20Reference) (OtherComp :type Primitive%20Component%20Object%20Reference) (OtherBodyIndex :type Integer))
  ;[1 1 1] Set "PlayerWithinRange" var
  (Utilities|Casting|CastToBP_Knight OtherActor)
  (Variables|Default|SetPlayerWithinRange false))

(event Custom|SwitchLight
  (if (Variables|Default|GetPlayerWithinRange)
    (Utilities|FlowControl|FlipFlop
      (:A
        (Rendering|SetVisibility (Variables|Default|GetTorch_PointLight) true false))
      (:B
        (Rendering|SetVisibility (Variables|Default|GetTorch_PointLight) false false)))))

(fn ConstructionScript)