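; BP_GoldCoins is a coin pickup actor that disappears when the third-person character overlaps it.
; CoinCollider's begin overlap calls CollectCoins, which destroys the three static mesh components and the collider but leaves the actor alive.
; The event then shows a BP_Coin widget and removes it after a short delay.
; ShowMessage and RemoveMessage go uncalled here, and RemoveMessage removes a newly created widget, not one already shown.
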(event OnComponentBeginOverlap(CoinCollider)
  (params (OverlappedComponent :type Primitive%20Component%20Object%20Reference) (OtherActor :type Actor%20Object%20Reference) (OtherComp :type Primitive%20Component%20Object%20Reference) (OtherBodyIndex :type Integer) (bFromSweep :type Boolean) (SweepResult :type Hit%20Result%20Structure%20%28by%20ref%29))
  (Utilities|Casting|CastToBP_ThirdPersonCharacter OtherActor)
  (CallFunction|CollectCoins)
  (bind _returnvalue (UserInterface|CreateWidget "/Game/ContentUsed/Widgets/BP_+Coin.BP_+Coin_C"))
  (UserInterface|Viewport|AddtoViewport _returnvalue 0)
  (Utilities|FlowControl|Delay 2.0)
  (Widget|RemovefromParent _returnvalue))

(fn ConstructionScript)

(fn CollectCoins
  (Components|DestroyComponent (Variables|Debug|GetStaticMeshComponent)) ; Makes the coins dissappear
  (Components|DestroyComponent (Variables|Default|GetStaticMeshComponent1)) ; Makes coin dissappear
  (Components|DestroyComponent (Variables|Default|GetStaticMeshComponent2)) ; Makes coins dissappear
  (Components|DestroyComponent (Variables|Default|GetCoinCollider)) ; Gets rid of collission box
)

(fn ShowMessage
  (bind _returnvalue (UserInterface|CreateWidget "/Game/ContentUsed/Widgets/BP_+Coin.BP_+Coin_C"))
  (UserInterface|Viewport|AddtoViewport _returnvalue 0))

(fn RemoveMessage
  (bind _returnvalue (UserInterface|CreateWidget "/Game/ContentUsed/Widgets/BP_+Coin.BP_+Coin_C"))
  (Widget|RemovefromParent _returnvalue))