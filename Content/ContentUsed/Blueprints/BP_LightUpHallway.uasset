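; BP_LightUpHallway is a trigger actor that lights up a hallway in sequence when the knight enters it.
; When BP_Knight overlaps the collision box, three groups of paired point lights and particle systems become visible one after another, separated by short delays.
; A spot light is revealed last, and nothing in the graph hides the lights again.
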(event OnComponentBeginOverlap(CollisionBox)
  (params (OverlappedComponent :type Primitive%20Component%20Object%20Reference) (OtherActor :type Actor%20Object%20Reference) (OtherComp :type Primitive%20Component%20Object%20Reference) (OtherBodyIndex :type Integer) (bFromSweep :type Boolean) (SweepResult :type Hit%20Result%20Structure%20%28by%20ref%29))
  (Utilities|Casting|CastToBP_Knight OtherActor)
  (Rendering|SetVisibility (Variables|Default|GetPointLight1) true false)
  (Utilities|FlowControl|Delay 1.0)
  (Rendering|SetVisibility (Variables|Default|GetPointLight3) true false)
  (Utilities|FlowControl|Delay 1.0)
  (Rendering|SetVisibility (Variables|Default|GetPointLight5) true false)
  (Utilities|FlowControl|Delay 1.0)
  (Rendering|SetVisibility (Variables|Default|GetSpotLight) true false))

(fn ConstructionScript)