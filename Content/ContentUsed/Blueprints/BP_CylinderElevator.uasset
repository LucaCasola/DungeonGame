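; BP_CylinderElevator is a cylinder elevator that carries the player up and back down once a lever has been activated.
; Third-person character overlap on its sphere triggers MoveComponentTo to raise the cylinder, pause briefly, then lower it, with eased timed moves.
; A looping-style 2D sound plays during each move and is stopped on arrival, while a CycleComplete flag blocks retriggering until the cycle ends.
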(event OnComponentBeginOverlap(CollisionSphere)
  (params (OverlappedComponent :type Primitive%20Component%20Object%20Reference) (OtherActor :type Actor%20Object%20Reference) (OtherComp :type Primitive%20Component%20Object%20Reference) (OtherBodyIndex :type Integer) (bFromSweep :type Boolean) (SweepResult :type Hit%20Result%20Structure%20%28by%20ref%29))
  (Utilities|Casting|CastToBP_ThirdPersonCharacter OtherActor)
  (if (Variables|Default|GetleverActivated)
    (if (Variables|Default|GetcycleComplete)
      (Variables|Default|SetcycleComplete false)
      (bind _returnvalue (Audio|SpawnSound2D "/Game/StarterContent/Audio/Light02.Light02" 1.0 1.0 0.0 0))
      (Variables|Default|Set2DSound _returnvalue)
      (Components|MoveComponentTo (Variables|Default|GetCylinder) "0.000000,0.000000,140.000000" "0, 0, 0" false true 5.0 false) ; Raises elevator
      (Audio|Components|Audio|Stop (Variables|Default|Get2DSound))
      (Utilities|FlowControl|Delay 3.0)
      (bind _returnvalue_2 (Audio|SpawnSound2D "/Game/StarterContent/Audio/Light02.Light02" 1.0 1.0 0.0 0))
      (Variables|Default|Set2DSound _returnvalue_2)
      (Components|MoveComponentTo (Variables|Default|GetCylinder) "0.000000,0.000000,-160.000000" "0, 0, 0" false true 5.0 false) ; Lowers elevator
      (Audio|Components|Audio|Stop (Variables|Default|Get2DSound))
      (Variables|Default|SetcycleComplete true))))

(fn ConstructionScript)