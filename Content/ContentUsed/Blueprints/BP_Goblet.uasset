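; BP_Goblet is a pickup actor that the third-person character collects by touching it.
; On overlap with BP_ThirdPersonCharacter, it destroys its cone and cylinder meshes and its collider, leaving the actor itself alive.
; It then shows a W_3Coin widget on screen and removes it after a short delay.
; The Blueprint changes no score or coin count itself.
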(event OnComponentBeginOverlap(GobletCollider)
  (params (OverlappedComponent :type Primitive%20Component%20Object%20Reference) (OtherActor :type Actor%20Object%20Reference) (OtherComp :type Primitive%20Component%20Object%20Reference) (OtherBodyIndex :type Integer) (bFromSweep :type Boolean) (SweepResult :type Hit%20Result%20Structure%20%28by%20ref%29))
  (Utilities|Casting|CastToBP_ThirdPersonCharacter OtherActor)
  (Components|DestroyComponent (Variables|Default|GetCone))
  (Components|DestroyComponent (Variables|Default|GetCone1))
  (Components|DestroyComponent (Variables|Default|GetCylinder))
  (Components|DestroyComponent (Variables|Default|GetGoblet%20Collider))
  (bind _returnvalue (UserInterface|CreateWidget "/Game/ContentUsed/Widgets/W_+3Coin.W_+3Coin_C"))
  (UserInterface|Viewport|AddtoViewport _returnvalue 0)
  (Utilities|FlowControl|Delay 2.0)
  (Widget|RemovefromParent _returnvalue))

(fn ConstructionScript)