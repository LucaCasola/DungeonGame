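; GameInstanceVarTracker holds copies of the player's Health and Gold so they can be saved and restored, apparently across level changes.
; StoreVariables copies both values from player 0's BP_ThirdPersonCharacter into tracker variables.
; LoadVariables writes the tracked values back onto the current character.
; Both events do nothing if the cast fails, and neither is triggered within this graph.
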(event Custom|Store%20Variables
  (bind _asbp_third_person_character (Utilities|Casting|CastToBP_ThirdPersonCharacter (Game|GetPlayerCharacter 0)))
  (Variables|Default|SetHealthTracker (Variables|/Game/ThirdPerson/Blueprints/BP_ThirdPersonCharacter.BP_ThirdPersonCharacter_C|GetHealth _asbp_third_person_character))
  (Variables|Default|SetGoldTracker (Variables|/Game/ThirdPerson/Blueprints/BP_ThirdPersonCharacter.BP_ThirdPersonCharacter_C|GetGold _asbp_third_person_character)))

(event Custom|Load%20Variables
  (bind _asbp_third_person_character (Utilities|Casting|CastToBP_ThirdPersonCharacter (Game|GetPlayerCharacter 0)))
  (Variables|/Game/ThirdPerson/Blueprints/BP_ThirdPersonCharacter.BP_ThirdPersonCharacter_C|SetHealth _asbp_third_person_character (Variables|Default|GetHealthTracker))
  (Variables|/Game/ThirdPerson/Blueprints/BP_ThirdPersonCharacter.BP_ThirdPersonCharacter_C|SetGold _asbp_third_person_character (Variables|Default|GetGoldTracker)))