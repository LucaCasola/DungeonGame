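; Barrel actor that loses health each time the third-person character enters its Box trigger.
; Each overlap subtracts one from BarHealth and flashes a W_Damage widget on screen for a fraction of a second.
; After that delay, if health is below one, it destroys the barrel mesh and trigger components, leaving the actor itself in place.
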(event OnComponentBeginOverlap(Box)
  (params (OverlappedComponent :type Primitive%20Component%20Object%20Reference) (OtherActor :type Actor%20Object%20Reference) (OtherComp :type Primitive%20Component%20Object%20Reference) (OtherBodyIndex :type Integer) (bFromSweep :type Boolean) (SweepResult :type Hit%20Result%20Structure%20%28by%20ref%29))
  (Utilities|Casting|CastToBP_ThirdPersonCharacter OtherActor)
  (Variables|Default|Setbar_health (- (Variables|Default|Getbar_health) 1))
  (bind _returnvalue (UserInterface|CreateWidget "/Game/ContentUsed/Widgets/W_Damage.W_Damage_C"))
  (UserInterface|Viewport|AddtoViewport _returnvalue 0)
  (Utilities|FlowControl|Delay 0.2)
  (Widget|RemovefromParent _returnvalue)
  (if (< (Variables|Default|Getbar_health) 1)
    (Components|DestroyComponent (Variables|Default|GetSM_Barrel))
    (Components|DestroyComponent (Variables|Default|GetBox))))

(fn ConstructionScript)