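; BP_GameState handles saving, loading and deleting the knight's progress in a single BP_SaveData slot.
; SaveGame reuses or creates the save object, then StoreData copies health, gold, necklace, transform and level name from BP_Knight and writes it.
; LoadGame restores stats and transform, then opens the saved level if it differs.
; LoadLevel restores only stats and necklace, without moving the player or changing levels.
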(event Custom|SaveGame
  ;[1 1 1] Save Game
  (bind _returnvalue (SaveGame|DoesSaveGameExist (Variables|Default|GetSaveSlotName)))
  (if _returnvalue
    (bind _returnvalue_2 (SaveGame|LoadGamefromSlot (Variables|Default|GetSaveSlotName)))
    (CallFunction|StoreData _returnvalue_2)
    (Development|PrintString "game saved!" true true "(R=0.000000,G=0.660000,B=1.000000,A=1.000000)" 1e+01)
    (else
      (bind _returnvalue_3 (SaveGame|CreateSaveGameObject "/Game/ContentUsed/Blueprints/SaveData/BP_SaveData.BP_SaveData_C"))
      (CallFunction|StoreData _returnvalue_3)
      (Development|PrintString "save file created!"))))

(event Custom|DeleteGame
  ;[1 1 1] Delete Game
  (bind _returnvalue (SaveGame|DoesSaveGameExist (Variables|Default|GetSaveSlotName)))
  (if _returnvalue
    (SaveGame|DeleteGameinSlot (Variables|Default|GetSaveSlotName))
    (Development|PrintString "Save deleted")))

(event Custom|LoadLevel
  ;[1 1 1] Load Level
  (bind _returnvalue (SaveGame|DoesSaveGameExist (Variables|Default|GetSaveSlotName)))
  (if _returnvalue
    (bind _returnvalue_2 (SaveGame|LoadGamefromSlot (Variables|Default|GetSaveSlotName)))
    (bind _output_get (Variables|Default|SetSaveFileRef _returnvalue_2))
    (bind _asbp_save_data (Utilities|Casting|CastToBP_SaveData _output_get))
    (bind _asbp_knight (Utilities|Casting|CastToBP_Knight (Game|GetPlayerCharacter 0)))
    (Variables|/Game/ContentUsed/PlayerCharacter/Blueprints/BP_Knight.BP_Knight_C|SetHealth _asbp_knight (Variables|/Game/ContentUsed/Blueprints/SaveData/BP_SaveData.BP_SaveData_C|GetHealth _asbp_save_data))
    (Variables|/Game/ContentUsed/PlayerCharacter/Blueprints/BP_Knight.BP_Knight_C|SetGold _asbp_knight (Variables|/Game/ContentUsed/Blueprints/SaveData/BP_SaveData.BP_SaveData_C|GetGold _asbp_save_data))
    (Variables|/Game/ContentUsed/PlayerCharacter/Blueprints/BP_Knight.BP_Knight_C|SetHasNecklace _asbp_knight (Variables|/Game/ContentUsed/Blueprints/SaveData/BP_SaveData.BP_SaveData_C|GetHasNecklace _asbp_save_data))
    (Default|AttachNecklace _asbp_knight)
    (else
      (Development|PrintString "failed to load save"))))

(event Custom|LoadGame
  ;[1 1 1] Load Game
  (bind _returnvalue (SaveGame|DoesSaveGameExist (Variables|Default|GetSaveSlotName)))
  (if _returnvalue
    (bind _returnvalue_2 (SaveGame|LoadGamefromSlot (Variables|Default|GetSaveSlotName)))
    (bind _output_get (Variables|Default|SetSaveFileRef _returnvalue_2))
    (bind _asbp_save_data (Utilities|Casting|CastToBP_SaveData _output_get))
    (bind _asbp_knight (Utilities|Casting|CastToBP_Knight (Game|GetPlayerCharacter 0)))
    (Variables|/Game/ContentUsed/PlayerCharacter/Blueprints/BP_Knight.BP_Knight_C|SetHealth _asbp_knight (Variables|/Game/ContentUsed/Blueprints/SaveData/BP_SaveData.BP_SaveData_C|GetHealth _asbp_save_data))
    (Variables|/Game/ContentUsed/PlayerCharacter/Blueprints/BP_Knight.BP_Knight_C|SetGold _asbp_knight (Variables|/Game/ContentUsed/Blueprints/SaveData/BP_SaveData.BP_SaveData_C|GetGold _asbp_save_data))
    (Variables|/Game/ContentUsed/PlayerCharacter/Blueprints/BP_Knight.BP_Knight_C|SetHasNecklace _asbp_knight (Variables|/Game/ContentUsed/Blueprints/SaveData/BP_SaveData.BP_SaveData_C|GetHasNecklace _asbp_save_data))
    (Default|AttachNecklace _asbp_knight)
    (Transformation|SetActorTransform (Game|GetPlayerCharacter 0) (Variables|/Game/ContentUsed/Blueprints/SaveData/BP_SaveData.BP_SaveData_C|GetPlayerTransform _asbp_save_data))
    (bind _returnvalue_3 (Game|GetCurrentLevelName true))
    (if (Utilities|Enum|NotEqual(Enum) _returnvalue_3 (Variables|/Game/ContentUsed/Blueprints/SaveData/BP_SaveData.BP_SaveData_C|GetCurrentLevel _asbp_save_data))
      (Game|OpenLevel(byName) (Utilities|String|StringToName (Variables|/Game/ContentUsed/Blueprints/SaveData/BP_SaveData.BP_SaveData_C|GetCurrentLevel _asbp_save_data))))
    (else
      (Development|PrintString "failed to load save"))))

(fn ConstructionScript)

(fn StoreData
  (params (SaveFileRef :type Save%20Game%20Object%20Reference))
  (bind _output_get (Variables|Default|SetSaveFileRef SaveFileRef))
  (bind _asbp_save_data (Utilities|Casting|CastToBP_SaveData _output_get))
  (Variables|Default|Setsave%20data _asbp_save_data)
  (bind _asbp_knight (Utilities|Casting|CastToBP_Knight (Game|GetPlayerCharacter 0)))
  (Variables|Default|Setplayer _asbp_knight)
  (Variables|/Game/ContentUsed/Blueprints/SaveData/BP_SaveData.BP_SaveData_C|SetHealth (Variables|Default|Getsave%20data) (Variables|/Game/ContentUsed/PlayerCharacter/Blueprints/BP_Knight.BP_Knight_C|GetHealth (Variables|Default|Getplayer)))
  (Variables|/Game/ContentUsed/Blueprints/SaveData/BP_SaveData.BP_SaveData_C|SetGold (Variables|Default|Getsave%20data) (Variables|/Game/ContentUsed/PlayerCharacter/Blueprints/BP_Knight.BP_Knight_C|GetGold (Variables|Default|Getplayer)))
  (Variables|/Game/ContentUsed/Blueprints/SaveData/BP_SaveData.BP_SaveData_C|SetHasNecklace (Variables|Default|Getsave%20data) (Variables|/Game/ContentUsed/PlayerCharacter/Blueprints/BP_Knight.BP_Knight_C|GetHasNecklace (Variables|Default|Getplayer)))
  (Variables|/Game/ContentUsed/Blueprints/SaveData/BP_SaveData.BP_SaveData_C|SetPlayerTransform (Variables|Default|Getsave%20data) (Transformation|GetActorTransform (Game|GetPlayerCharacter 0)))
  (bind _returnvalue (Game|GetCurrentLevelName true))
  (Variables|/Game/ContentUsed/Blueprints/SaveData/BP_SaveData.BP_SaveData_C|SetCurrentLevel (Variables|Default|Getsave%20data) _returnvalue)
  (SaveGame|SaveGametoSlot (Variables|Default|GetSaveFileRef) (Variables|Default|GetSaveSlotName)))