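; BP_Barrel is a breakable barrel with a mesh, a collision component and a health counter.
; Overlap events on the collision component set an in-range flag while a BP_ThirdPersonCharacter is inside.
; Damage logic lowers health by one when in range and calls KillBarrel below one to destroy both components, but no event triggers it.
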(event OnComponentBeginOverlap(BarrelCollision)
  (params (OverlappedComponent :type Primitive%20Component%20Object%20Reference) (OtherActor :type Actor%20Object%20Reference) (OtherComp :type Primitive%20Component%20Object%20Reference) (OtherBodyIndex :type Integer) (bFromSweep :type Boolean) (SweepResult :type Hit%20Result%20Structure%20%28by%20ref%29))
  ;[1 1 1] While the user is in range, set in range to true, else set false
  (Utilities|Casting|CastToBP_ThirdPersonCharacter OtherActor)
  (Variables|Default|SetinRange true))

(event OnComponentEndOverlap(BarrelCollision)
  (params (OverlappedComponent :type Primitive%20Component%20Object%20Reference) (OtherActor :type Actor%20Object%20Reference) (OtherComp :type Primitive%20Component%20Object%20Reference) (OtherBodyIndex :type Integer))
  ;[1 1 1] While the user is in range, set in range to true, else set false
  (Utilities|Casting|CastToBP_ThirdPersonCharacter OtherActor)
  (Variables|Default|SetinRange false))

(fn ConstructionScript)

(fn KillBarrel
  (Components|DestroyComponent (Variables|Default|GetSM_Barrel))
  (Components|DestroyComponent (Variables|Default|GetBarrelCollision)))